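; HunterRaptor_Character_BP is a raptor creature that caps how many of its kind exist at once.
; Shortly after BeginPlay, dedicated and player-hosted servers read MaxRaptors from the game mode's DinoHunter ini section, with a fallback for non-positive values.
; It then counts all actors of its class and destroys itself, rather than the surplus array entries, if the count exceeds that limit.
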(event `self.ReceiveBeginPlay`
  (`KismetSystemLibrary.Delay` 0.2)
  (`/Engine/EditorBlueprintResources/ActorMacros.SwitchNetAuthority`
    (:`DedicatedServer`
      _)
    (:`PlayerServer`
      _))
  (bind _asshootergamemode (cast `ShooterGameMode` (`GameplayStatics.GetGameMode`)))
  (bind _returnvalue (`ShooterGameMode.GetFloatOptionIni` _asshootergamemode "DinoHunter" "MaxRaptors"))
  (bind _returnvalue_2 (`KismetMathLibrary.FFloor` _returnvalue))
  (if (<= _returnvalue_2 0)
    (set `self.MaxAllowed` 5)
    (else
      (set `self.MaxAllowed` _returnvalue_2)))
  (bind _outactors (`GameplayStatics.GetAllActorsOfClass` "HunterRaptor_Character_BP_C"))
  (for (_ _array_index) _outactors
    (if (not (< _array_index (`self.MaxAllowed`)))
      (`self.K2_DestroyActor`))))

(fn `UserConstructionScript`
  (`parent.UserConstructionScript`))
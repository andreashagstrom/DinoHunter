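; HunterBat creature character that caps its own population and can infect characters it hits with rabies.
; Shortly after spawning on a server, it reads the MaxBats INI option, falling back to a default, and destroys itself if the bat count exceeds that cap.
; Each attack check re-arms a single infection attempt, which the damage hook spends on a server-side random roll to apply Buff_ReptileRabies, leaving damage unchanged.
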(event `self.ReceiveBeginPlay`
  (`KismetSystemLibrary.Delay` 0.2)
  (`/Engine/EditorBlueprintResources/ActorMacros.SwitchNetAuthority`
    (:`DedicatedServer`
      _)
    (:`PlayerServer`
      _))
  (bind _asshootergamemode (cast `ShooterGameMode` (`GameplayStatics.GetGameMode`)))
  (bind _returnvalue (`ShooterGameMode.GetFloatOptionIni` _asshootergamemode "DinoHunter" "MaxBats"))
  (bind _returnvalue_2 (`KismetMathLibrary.FFloor` _returnvalue))
  (if (<= _returnvalue_2 0)
    (set `self.MaxAllowed` 5)
    (else
      (set `self.MaxAllowed` _returnvalue_2)))
  (bind _outactors (`GameplayStatics.GetAllActorsOfClass` "HunterBat_Character_BP_C"))
  (for (_ _array_index) _outactors
    (if (not (< _array_index (`self.MaxAllowed`)))
      (`self.K2_DestroyActor`))))

(fn `BlueprintAdjustOutputDamage`
  (params (AttackIndex :type Integer) (OriginalDamageAmount :type "Float (double-precision)") (HitActor :type "Actor Object Reference"))
  (returns (OutDamageType :type "DamageType Class Reference") (OutDamageImpulse :type "Float (double-precision)") (ReturnValue :type "Float (double-precision)"))
  (bind (_attackname _attackweight _attackrange _minattackrange _activateattackrange _attackinterval _bhighqualityattack _bskipuntamed _bskiptamed _bonlyonwilddinos _bpreventwhenencumbered _bridingonlyallowonground _bridingonlyallowwhileflying _bonlyusewithplayersorriders _bonlyusewithplayers _bpreventwhenswimming _bpreventwheninsufficientstamina _bskiponflyers _bskipai _bpreventonfemale _bpreventonmale _bpreventwhendinocarrying _buseblueprintcanriderattack _brequireswalking _brequiresswimming _attackstatusstarted _battackstopsmovement _battackstopsmovementallowfalling _battackwithjump _blocationbasedattack _bdropcarriedcharacter _bcancelanddropifcarriedcharacter _bpreventattackwhilerunning _forceupdateinrange _forceupdatemeshself _busesecondaryanimationinair _buseblueprintcanattack _buseblueprintadjustoutputdamage _bdisablerunningwhenattacking _bkeepexecutingwhenacquiringtarget _bpreventwithrider _baiforceattackdotproductcheck _binstantlyharvestcorpse _baddpawnvelocitytoprojectile _battackstopsrotation _btamedaispecialattack _bpreventwhencarryingexplosive _ballowwhenanimationpreventsinput _brequirelineofsight _busesecondaryanimationwhenswimming _busetertiaryanimationwhenswimming _bhighqualityattackonlyplayerortamed _childstateindexes _attackwithjumpchance _lastattacktime _riderlastattacktime _attackselectionexpirationtime _attackselectiontime _attackrotationrangedegrees _attackrotationgroundspeedmultiplier _attackrotationrate _meleeswingsockets _rangedsocket _meleedamageamount _meleedamageimpulse _meleeswingradius _meleedamagetype) (break `PrimalDinoCharacter.DinoAttackInfo` (`KismetArrayLibrary.Array_Get` (`self.AttackInfos`) AttackIndex)))
  (`|ExecutionSequence`
    (:`then_0`
      (`/Engine/EditorBlueprintResources/StandardMacros.IsValid` HitActor
        (:`Is Valid`
          (bind _asprimalcharacter (cast `PrimalCharacter` HitActor))
          (if (`self.bCanTryGiveRabies`)
            (set `self.bCanTryGiveRabies` false)
            (if (and (`KismetSystemLibrary.IsServer`) (>= (`KismetMathLibrary.RandomFloat`) (- 1.0 (`self.ChanceForMegaRabies`))))
              (`PrimalBuff.StaticAddBuff` "/Game/PrimalEarth/CoreBlueprints/Buffs/Buff_ReptileRabies.Buff_ReptileRabies_C" _asprimalcharacter null self))))))
    (:`then_1`
      (return _meleedamagetype _meleedamageimpulse OriginalDamageAmount))))

(fn `BlueprintCanAttack`
  (params (AttackIndex :type Integer) (distance :type "Float (double-precision)") (attackRangeOffset :type "Float (double-precision)") (OtherTarget :type "Actor Object Reference"))
  (returns (ReturnValue :type Boolean))
  (set `self.bCanTryGiveRabies` true)
  (return true))

(fn `UserConstructionScript`
  (`parent.UserConstructionScript`))
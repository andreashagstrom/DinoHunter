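; Hunter variant of the Kaprosuchus creature, built around a leap attack that grabs and holds prey on land or in water.
; Anim notifies launch a replicated impulse scaled by slope and water depth; landing clears the leap, carries momentum briefly and starts the grab.
; Movement mode swaps attack animation weights, while timers release dead or unconscious prey.
; On servers, BeginPlay self-destroys when instances exceed an INI-configured limit.
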(event Custom|StopHoldingCharacter
  ;[0.9428 0 1] LeapGrab and StopHolding
  (for _array_element (Class|PrimalCharacter|GetBuffs)
    (bind _asbuff_isbeingcarried_c (Utilities|Casting|CastToBuff_IsBeingCarried _array_element))
    (Variables|/Script/ShooterGame.PrimalBuff|SetDeactivateAfterTime _asbuff_isbeingcarried_c 0.0))
  (Variables|Local/Temp|SetbIsHoldingCharacter false)
  (Animation|StopAnimMontage "/Game/PrimalEarth/Dinos/Kaprosuchus/Animations/Kaprosuchus-Attack-Grab-Chew_Montage.Kaprosuchus-Attack-Grab-Chew_Montage")
  (Class|PrimalCharacter|PlayAnimEx "/Game/PrimalEarth/Dinos/Kaprosuchus/Animations/Kaprosuchus-Attack-Grab-Drop_Montage.Kaprosuchus-Attack-Grab-Drop_Montage" 1.0 "None" false false false false))

(event Custom|Multi_StopHoldingCharacter
  ;[0.9428 0 1] LeapGrab and StopHolding
  (CallFunction|StopHoldingCharacter))

(event Custom|ContinueMomentum
  ;[1 1 1] Velocity preservation to help smooth landings on water or other surfaces
  (Variables|/Script/Engine.MovementComponent|SetVelocity (Variables|Character|GetCharacterMovement) (* (Variables|Local/Temp|GetInitialLungeVelocity) (Math|Float|SelectFloat 1.0 0.4 (Class|PrimalCharacter|IsSubmerged false false false false)))))

(event Custom|SetIgnoreMoveInput
  ;[1 1 1] Velocity preservation to help smooth landings on water or other surfaces
  (Variables|Local/Temp|SetbShouldIgnoreMoveInput false)
  (Utilities|Time|ClearTimerbyFunctionName self "ContinueMomentum")
  (Variables|Local/Temp|SetInitialLungeVelocity "0, 0, 0"))

(event Custom|StartGrab
  ;[0.9428 0 1] LeapGrab and StopHolding
  (Utilities|IsValid (Variables|Default|GetCarriedCharacter)
    (:Is%20Valid
      (Variables|Local/Temp|SetbIsHoldingCharacter true)
      (Class|PrimalCharacter|PlayAnimEx "/Game/PrimalEarth/Dinos/Kaprosuchus/Animations/Kaprosuchus-Attack-Grab-Chew_Montage.Kaprosuchus-Attack-Grab-Chew_Montage" 1.0 "None" false false false false))))

(event Custom|AnimNotify_StartLeapAttack
  ;[0 1 0.0172] StartLeap
  (Utilities|FlowControl|DoOnce false
    (:Completed
      (Utilities|FlowControl|Sequence
        (:then_0
          (Variables|Local/Temp|SetbIsFallingFromLeap true)
          (Variables|Default|SetRootLocSwimOffset 0.0)
          (Variables|Local/Temp|SetbShouldIgnoreMoveInput true))
        (:then_1
          (bind _nearsurface (CallFunction|EvaluateHeightinWater))
          (Utilities|FlowControl|Delay (Math|Float|SelectFloat 0.3 (Variables|Default|GetSubmergedIgnoreWaterTime) (or _nearsurface (not (Class|PrimalCharacter|IsSubmerged false false false false)))))
          (Variables|Default|SetbCanIgnoreWater false false))
        (:then_2
          (if (not (Networking|IsDedicatedServer))
            (CallFunction|PlayLeapFX (Math|Conversions|ToInteger(Byte) (Variables|/Script/Engine.CharacterMovementComponent|GetMovementMode (Variables|Character|GetCharacterMovement))) true)))
        (:then_3
          (CallFunction|SetLeapRotation)
          (Variables|/Script/Engine.MovementComponent|SetVelocity (Variables|Character|GetCharacterMovement) "0, 0, 0")
          (bind _retimpulse (CallFunction|CalcLeapImpulse))
          (Variables|Default|SetbCanIgnoreWater true false)
          (Class|PrimalCharacter|BPNetAddCharacterMovementImpulse _retimpulse true 1.0 true "MOVE_Falling" false false)
          (Networking|ForceNetUpdate)
          (Utilities|FlowControl|Delay 0.2)
          (Variables|Local/Temp|SetInitialLungeVelocity (Variables|/Script/Engine.MovementComponent|GetVelocity (Variables|Character|GetCharacterMovement))))))))

(event Custom|AnimNotify_StartLeapGrab
  ;[0.9428 0 1] LeapGrab and StopHolding
  (Utilities|IsValid (Variables|Default|GetCarriedCharacter)
    (:Is%20Valid
      (Variables|Local/Temp|SetbIsHoldingCharacter true)
      (Class|PrimalCharacter|PlayAnimEx "/Game/PrimalEarth/Dinos/Kaprosuchus/Animations/Kaprosuchus-Attack-Grab-Chew_Montage.Kaprosuchus-Attack-Grab-Chew_Montage" 1.0 "None" false false false false))))

(event Custom|AnimNotify_EndLeap
  ;[0.1254 0.1394 1] EndLeap
  (Variables|Default|SetbCanIgnoreWater false false)
  (if (Variables|Local/Temp|GetbIsFallingFromLeap)
    (CallFunction|ClearLeapAttack -1)))

(event Custom|Multi_ClearLeap
  (params (IsWalking :type Boolean))
  ;[0 0.5239 1] Clear Leap Attack
  (Variables|Default|SetbCanIgnoreWater false false)
  (Variables|Local/Temp|SetbIsFallingFromLeap false)
  (Class|PrimalCharacter|PlayAnimEx (select IsWalking "/Game/PrimalEarth/Dinos/Kaprosuchus/Animations/Kaprosuchus-Lunge-Out-Ground_Montage.Kaprosuchus-Lunge-Out-Ground_Montage" "/Game/PrimalEarth/Dinos/Kaprosuchus/Animations/Kaprosuchus-Lunge-Out-Swim_Montage.Kaprosuchus-Lunge-Out-Swim_Montage") 1.0 "None" true false false false)
  (CallFunction|StartGrab)
  (bind _returnvalue (Class|VictoryCore|GetDefaultObject self))
  (bind _asprimaldinocharacter (Utilities|Casting|CastToPrimalDinoCharacter _returnvalue))
  (Variables|Default|SetRootLocSwimOffset (Variables|/Script/ShooterGame.PrimalDinoCharacter|GetRootLocSwimOffset _asprimaldinocharacter))
  (CallFunction|ResetStartLeap)
  (Utilities|FlowControl|Sequence
    (:then_0
      (Utilities|Time|SetTimerbyFunctionName self "SetIgnoreMoveInput" (Math|Float|SelectFloat 0.15 0.2 (not (Class|PrimalCharacter|IsSubmerged false false false false))))
      (Utilities|Time|SetTimerbyFunctionName self "ContinueMomentum" 0.01 true))
    (:then_1
      (if (not (Networking|IsDedicatedServer))
        (CallFunction|PlayLeapFX (select IsWalking 1 3) false)))))

(event Custom|ClearLeapAttack
  (params (LandingInMovementMode :type Integer))
  ;[0 0.5239 1] Clear Leap Attack
  (CallFunction|MultiClearLeap (== LandingInMovementMode 1)))

(event Custom|ResetStartLeap
  ;[0 1 0.0172] StartLeap
  (Utilities|FlowControl|DoOnce false) ; enters at Reset
)

(event EventBeginPlay
  (Utilities|FlowControl|Delay 0.2)
  (Utilities|SwitchNetAuthority
    (:DedicatedServer
      _)
    (:PlayerServer
      _))
  (bind _asshootergamemode (Utilities|Casting|CastToShooterGameMode (Game|GetGameMode)))
  (bind _returnvalue (Class|ShooterGameMode|GetFloatOptionIni _asshootergamemode "DinoHunter" "MaxKapros"))
  (if (<= (Math|Float|Floor _returnvalue) 0)
    (Variables|Default|SetMaxAllowed 5)
    (else
      (Variables|Default|SetMaxAllowed (Math|Float|Floor _returnvalue))))
  (bind _outactors (Actor|GetAllActorsOfClass "HunterKaprosuchus_Character_BP_C"))
  (for (_ _array_index) _outactors
    (if (not (< _array_index (Variables|Default|GetMaxAllowed)))
      (Actor|DestroyActor))))

(fn ConstructionScript
  (|CallParentFunction))

(fn SetLeapRotation
  (bind _returnvalue (Transformation|GetActorRotation))
  (bind _returnvalue_2 (Transformation|GetActorRotation))
  (bind _target (Variables|Default|GetTarget))
  (bind _leapangleturnallowance (Variables|Default|GetLeapAngleTurnAllowance))
  (bind _leapangleturnallowance_2 (Variables|Default|GetLeapAngleTurnAllowance))
  (bind _yaw (Class|KismetMathLibrary|BreakRot _returnvalue))
  (bind _yaw_2 (Class|KismetMathLibrary|BreakRot _returnvalue_2))
  (if (Variables|Default|GetbHasRider)
    (Transformation|SetActorRotation (Class|KismetMathLibrary|MakeRot 0.0 (Math|Float|Clamp(Float) (.Yaw (Class|KismetMathLibrary|BreakRot (Pawn|GetBaseAimRotation))) (- _yaw_2 _leapangleturnallowance_2) (+ _yaw_2 _leapangleturnallowance_2)) 0.0))
    (else
      (Utilities|IsValid _target
        (:Is%20Valid
          (Transformation|SetActorRotation (Class|KismetMathLibrary|MakeRot 0.0 (Math|Float|Clamp(Float) (.Yaw (Class|KismetMathLibrary|BreakRot (Math|Rotator|FindLookatRotation (Transformation|GetActorLocation) (Transformation|GetActorLocation _target)))) (- _yaw _leapangleturnallowance) (+ _yaw _leapangleturnallowance)) 0.0)))))))

(fn BPonMovementModeChangedNotify
  (params (PrevMovementMode :type EMovementMode%20Enum :default "MOVE_None") (PreviousCustomMode :type Byte :default 0))
  (|CallParentFunction "MOVE_None" 0)
  (switch Utilities|FlowControl|Switch|SwitchonEMovementMode (Variables|/Script/Engine.CharacterMovementComponent|GetMovementMode (Variables|Character|GetCharacterMovement))
    (:MOVE_None
      (CallFunction|ChangeGroundSwimAttackAnims (Math|Integer|SelectInt 0 1 (Utilities|Enum|Equal(Enum) (Variables|/Script/Engine.CharacterMovementComponent|GetMovementMode (Variables|Character|GetCharacterMovement)) "MOVE_Walking")) :!label _label))
    (:MOVE_Walking
      (Utilities|FlowControl|Sequence :!label _label_2
        (:then_0
          (goto _label))
        (:then_1
          (if (Variables|Local/Temp|GetbIsFallingFromLeap)
            (CallFunction|ClearLeapAttack (Math|Conversions|ToInteger(Byte) (Variables|/Script/Engine.CharacterMovementComponent|GetMovementMode (Variables|Character|GetCharacterMovement))))))))
    (:MOVE_Falling
      (goto _label))
    (:MOVE_Swimming
      (goto _label_2))
    (:MOVE_Flying
      (goto _label))
    (:MOVE_Custom
      (goto _label))))

(fn BPTimerNonDedicated
  (bind _carriedcharacter (Variables|Default|GetCarriedCharacter))
  (Variables|Default|SetClientLocationInterpSpeed (select (and (Utilities|Enum|Equal(Enum) (Variables|/Script/Engine.CharacterMovementComponent|GetMovementMode (Variables|Character|GetCharacterMovement)) "MOVE_Falling") (Variables|Local/Temp|GetbIsFallingFromLeap)) 1e+02 7.0))
  (if (Variables|Local/Temp|GetbIsHoldingCharacter)
    (if (Math|Boolean|ORBoolean (not (Utilities|IsValid _carriedcharacter)) (not (Class|PrimalCharacter|BPIsConscious _carriedcharacter)) (not (Class|PrimalCharacter|BPIsConscious)))
      (CallFunction|StopHoldingCharacter))))

(fn ChangeGroundSwimAttackAnims
  (params (NewState :type Integer))
  (bind _attackinfos (Variables|Default|GetAttackInfos))
  (bind _item (Utilities|Array|Get(acopy) _attackinfos))
  (bind _attackanimationweights (Utilities|Struct|BreakDinoAttackInfo _item))
  (bind _item_2 (Utilities|Array|Get(acopy) _attackanimationweights))
  (bind _returnvalue (Math|Float|NearlyEqual(Float) _item_2 1.0 1e-06))
  (switch int NewState
    (:0
      ;[1 1 1] Move to Land
      (if (not _returnvalue)
        (Class|PrimalDinoCharacter|CycleAttackWeightsforAttackatIndex)
        (Class|PrimalDinoCharacter|CycleAttackWeightsforAttackatIndex 1)
        (Class|PrimalDinoCharacter|CycleAttackWeightsforAttackatIndex 2)))
    (:1
      ;[1 1 1] Move to Water
      (if _returnvalue
        (Class|PrimalDinoCharacter|CycleAttackWeightsforAttackatIndex)
        (Class|PrimalDinoCharacter|CycleAttackWeightsforAttackatIndex 1)
        (Class|PrimalDinoCharacter|CycleAttackWeightsforAttackatIndex 2)))))

(fn BlueprintCanAttack
  (params (AttackIndex :type Integer) (distance :type Float%20%28single-precision%29) (attackRangeOffset :type Float%20%28single-precision%29) (OtherTarget :type Actor%20Object%20Reference))
  (bind _returnvalue (== AttackIndex 1))
  (LocalVariables|SetretVal true)
  (Utilities|FlowControl|Sequence
    (:then_0
      (if (or _returnvalue (== AttackIndex 2))
        (LocalVariables|SetretVal (not (Utilities|IsValid (Variables|Default|GetCarriedCharacter))))))
    (:then_1
      (if (and _returnvalue (Utilities|Enum|Equal(Enum) (Variables|/Script/Engine.CharacterMovementComponent|GetMovementMode (Variables|Character|GetCharacterMovement)) "MOVE_Swimming"))
        (bind _returnvalue_2 (Transformation|GetDistanceTo (Variables|Default|GetTarget)))
        (LocalVariables|SetretVal (and (<= _returnvalue_2 (Variables|Default|GetLeapWaterAttackRange)) (>= _returnvalue_2 (Variables|Default|GetLeapWaterMinAttackRange))))))
    (:then_2
      (return (LocalVariables|GetretVal)))))

(fn CalcLeapImpulse
  (bind _mesh (Variables|Character|GetMesh))
  (bind _mesh_2 (Variables|Character|GetMesh))
  (bind _returnvalue (Transformation|GetWorldLocation _mesh))
  (bind _returnvalue_2 (Transformation|GetWorldLocation _mesh_2))
  (LocalVariables|SetTrueForward (Transformation|GetActorForwardVector))
  (if (Variables|Default|GetbUseSlopeSensitiveLeap)
    (|FindPitchSensitiveForward
      (:OutputPin
        _)))
  (bind _nearsurface (CallFunction|EvaluateHeightinWater))
  (LocalVariables|SetRetValImpulse (* (* (|ApplyWater/GroundMultipliers (Math|Vector|GetForwardVector (Class|KismetMathLibrary|MakeRot (Math|Float|Clamp(Float) (+ (Variables|Default|GetLeapAdditionalPitch) (.Pitch (Class|KismetMathLibrary|BreakRot (Math|Rotator|MakeRotfromX (LocalVariables|GetTrueForward))))) -2e+01 9e+01) (.Yaw (Class|KismetMathLibrary|BreakRot (Math|Rotator|MakeRotfromX (LocalVariables|GetTrueForward)))) (.Roll (Class|KismetMathLibrary|BreakRot (Math|Rotator|MakeRotfromX (LocalVariables|GetTrueForward)))))) _nearsurface) (Math|Vector|MakeVector 1.0 1.0 (+ (* (Math|Float|Power (Math|Float|Absolute(Float) (/ (Math|Float|Clamp(Float) (+ (Variables|Default|GetLeapAdditionalPitch) (.Pitch (Class|KismetMathLibrary|BreakRot (Math|Rotator|MakeRotfromX (LocalVariables|GetTrueForward))))) -2e+01 9e+01) 9e+01)) 0.2) (Variables|Default|GetLeapSlopeAngleMultiplier)) 1.0))) (Variables|Default|GetLeapImpulse)))
  (if (Variables|Default|GetbDebugKaproAbilities)
    (Rendering|Debug|DrawDebugArrow _returnvalue (+ _returnvalue (* (LocalVariables|GetTrueForward) 1e+02)) 5e+02 "(R=0.840000,G=0.314406,B=0.077633,A=1.000000)" 5e+01)
    (Rendering|Debug|DrawDebugArrow _returnvalue_2 (+ _returnvalue_2 (* (Math|Vector|Normalize (LocalVariables|GetRetValImpulse)) 1e+02)) 5e+02 "(R=0.000000,G=0.000000,B=0.000000,A=1.000000)" 5e+01)
    (Development|PrintString (Utilities|String|Append "Leap data: " (Utilities|String|ToString(Rotator) (Class|KismetMathLibrary|MakeRot (Math|Float|Clamp(Float) (+ (Variables|Default|GetLeapAdditionalPitch) (.Pitch (Class|KismetMathLibrary|BreakRot (Math|Rotator|MakeRotfromX (LocalVariables|GetTrueForward))))) -2e+01 9e+01) (.Yaw (Class|KismetMathLibrary|BreakRot (Math|Rotator|MakeRotfromX (LocalVariables|GetTrueForward)))) (.Roll (Class|KismetMathLibrary|BreakRot (Math|Rotator|MakeRotfromX (LocalVariables|GetTrueForward)))))))))
  (return (LocalVariables|GetRetValImpulse)))

(fn BlueprintCanRiderAttack
  (params (AttackIndex :type Integer))
  (bind _returnvalue (== AttackIndex 1))
  (bind _attackinfos (Variables|Default|GetAttackInfos))
  (bind _item (Utilities|Array|Get(acopy) _attackinfos AttackIndex))
  (bind (_attackname _attackweight _attackrange _minattackrange _activateattackrange _attackinterval _bhighqualityattack _bskipuntamed _bskiptamed _bonlyonwilddinos _bpreventwhenencumbered _bridingonlyallowonground _bridingonlyallowwhileflying _bonlyusewithplayersorriders _bonlyusewithplayers _bpreventwhenswimming _bpreventwheninsufficientstamina _bskiponflyers _bskipai _bpreventonfemale _bpreventonmale _bpreventwhendinocarrying _buseblueprintcanriderattack _brequireswalking _brequiresswimming _attackstatusstarted _battackstopsmovement _battackstopsmovementallowfalling _battackwithjump _blocationbasedattack _bdropcarriedcharacter _bcancelanddropifcarriedcharacter) (Utilities|Struct|BreakDinoAttackInfo _item))
  (LocalVariables|SetretVal true)
  (Utilities|FlowControl|Sequence
    (:then_0
      (if _returnvalue
        (LocalVariables|SetretVal (not (Utilities|IsValid (Variables|Default|GetCarriedCharacter))))))
    (:then_1
      (if (or _bdropcarriedcharacter _bcancelanddropifcarriedcharacter)
        (if (Utilities|IsValid (Variables|Default|GetCarriedCharacter))
          (LocalVariables|SetretVal true)
          (CallFunction|StopHoldingCharacter))))
    (:then_2
      (if (and _returnvalue (Variables|Local/Temp|GetbIsFallingFromLeap))
        (LocalVariables|SetRetVal false)))
    (:then_3
      (return (LocalVariables|GetretVal)))))

(fn BPTimerServer
  (bind _carriedcharacter (Variables|Default|GetCarriedCharacter))
  (if (Variables|Local/Temp|GetbIsHoldingCharacter)
    (if (Math|Boolean|ORBoolean (not (Utilities|IsValid _carriedcharacter)) (not (Class|PrimalCharacter|BPIsConscious _carriedcharacter)) (not (Class|PrimalCharacter|BPIsConscious)))
      (CallFunction|StopHoldingCharacter))))

(fn BPModifyForwardDirectionInput
  (params (directionInput :type Vector%20%28by%20ref%29 :default "0, 0, 0"))
  (return "0, 0, 0"))

(fn BPShouldLimitForwardDirection
  (return (Variables|Local/Temp|GetbShouldIgnoreMoveInput)))

(fn EvaluateHeightinWater
  (bind _returnvalue (Transformation|GetActorLocation))
  (LocalVariables|SetRetVal false)
  (bind (_outhits _returnvalue_2) (Class|VictoryCore|VTraceMultiBP (Class|Actor|GetWorld) (+ _returnvalue "0, 0,150.000000") (- _returnvalue "0, 0,60.000000") 0 -1 1.0 (Math|Vector|MakeVector 0.0 0.0 0.0) false "ECC_WorldStatic" false "None" true false 0 0 false))
  (if _returnvalue_2
    (for _array_element _outhits
      (bind _asphysicsvolume (Utilities|Casting|CastToPhysicsVolume (.HitActor (Collision|BreakHitResult _array_element))))
      (if (Variables|/Script/Engine.PhysicsVolume|GetbWaterVolume _asphysicsvolume)
        (if (<= (Math|Vector|VectorLength (- (.Location (Collision|BreakHitResult _array_element)) (Transformation|GetActorLocation))) (Variables|/Script/Engine.CapsuleComponent|GetCapsuleHalfHeight (Variables|Default|GetCapsuleComponent)))
          (LocalVariables|SetRetVal true))))
    (return (LocalVariables|GetRetVal))))

(fn PlayLeapFX
  (params (MovementMode :type Integer) (IsLeapStart :type Boolean))
  (switch int MovementMode
    (:1
      (if (not (Class|PrimalCharacter|IsSubmerged false false false false))
        (Effects|SpawnEmitterAttached (Variables|Default|GetLeapGroundImpactParticle) (Variables|Character|GetMesh) "GroundFX")
        (else
          (bind _nearsurface (CallFunction|EvaluateHeightinWater :!label _label))
          (Effects|SpawnEmitterAttached (select IsLeapStart (select _nearsurface (Variables|Default|GetLeapWaterSurfaceStartParticle) (Variables|Default|GetLeapWaterSubmergedStartParticle)) (select _nearsurface (Variables|Default|GetLeapWaterSurfaceEndParticle) (Variables|Default|GetLeapWaterSubmergedEndParticle))) (Variables|Character|GetMesh) "GroundFX"))))
    (:3
      (goto _label))))

(fn BPGetMultiUseEntries
  (params (ForPC :type Player%20Controller%20Object%20Reference) (MultiUseEntries :type Array%20of%20Multi%20Use%20Entry%20Structures))
  (if (and (or (== (Variables|/Script/Engine.Actor|GetTargetingTeam ForPC) (Variables|Default|GetTargetingTeam)) (not (Class|PrimalCharacter|BPIsConscious))) (Utilities|IsValid (Variables|Default|GetCarriedCharacter)))
    (Utilities|Array|Add MultiUseEntries (Utilities|Struct|MakeMultiUseEntry 0 "Drop Prey" 26060)))
  (return MultiUseEntries))

(fn BPTryMultiUse
  (params (ForPC :type Player%20Controller%20Object%20Reference) (UseIndex :type Integer))
  (switch int UseIndex
    (:Default
      _)
    (:26060
      (Class|PrimalDinoCharacter|ClearCarriedCharacter false false)
      (CallFunction|StopHoldingCharacter)))
  (return true))
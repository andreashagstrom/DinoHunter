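; Hunter Megalodon shark character that limits its own population and supports Tek helmet zoom.
; Shortly after BeginPlay on dedicated or player servers, it reads MaxSharks from the DinoHunter ini section, defaulting to five if not positive.
; It counts all actors of its class and destroys itself if they exceed that cap.
; BPModifyFOV narrows the view when a Tek helmet buff has targeting mode enabled.
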(event EventBeginPlay
  (Utilities|FlowControl|Delay 0.2)
  (Utilities|SwitchNetAuthority
    (:DedicatedServer
      _)
    (:PlayerServer
      _))
  (bind _asshootergamemode (Utilities|Casting|CastToShooterGameMode (Game|GetGameMode)))
  (bind _returnvalue (Class|ShooterGameMode|GetFloatOptionIni _asshootergamemode "DinoHunter" "MaxSharks"))
  (if (<= (Math|Float|Floor _returnvalue) 0)
    (Variables|Default|SetMaxAllowed 5)
    (else
      (Variables|Default|SetMaxAllowed (Math|Float|Floor _returnvalue))))
  (bind _outactors (Actor|GetAllActorsOfClass "HunterMegalodon_Character_BP_C"))
  (for (_ _array_index) _outactors
    (if (not (< _array_index (Variables|Default|GetMaxAllowed)))
      (Actor|DestroyActor))))

(fn ConstructionScript
  (|CallParentFunction))

(fn BPModifyFOV
  (params (FOVIn :type Float%20%28single-precision%29))
  (LocalVariables|SetretVal FOVIn)
  (Utilities|FlowControl|Sequence
    (:then_0
      (bind _array_element (Utilities|Array|ForEachLoopwithBreak (Class|PrimalCharacter|GetBuffs) :!label _label)
        (:LoopBody
          (bind _asbuff_dinotekhelmet_base_c (Utilities|Casting|CastToBuff_DinoTekHelmet_Base _array_element))
          (if (Variables|/Game/PrimalEarth/CoreBlueprints/Buffs/Buff_DinoTekHelmet_Base.Buff_DinoTekHelmet_Base_C|GetbIsTargetingModeEnabled _asbuff_dinotekhelmet_base_c)
            (LocalVariables|SetretVal 55.0)
            (goto _label Break)
            (else
              (goto _label Break))))))
    (:then_1
      (return (LocalVariables|GetretVal)))))
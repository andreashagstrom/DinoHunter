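; Hunter Mantis creature whose signature move is a leap attack, with instance count capped by a DinoHunter INI setting at BeginPlay.
; An anim notify launches a flying impulse along the slope or toward its target.
; A server timer applies multicast downforce and checks for the end; overlaps or bumps deal direct damage, and finishing deals radial damage.
; An equipped glove-slot weapon modifies melee damage and harvesting, losing durability on regular attacks.
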(event OnComponentBeginOverlap(AttackCheckSphere)
  (params (OtherActor :type Actor%20Object%20Reference) (OtherComp :type Primitive%20Component%20Object%20Reference) (OtherBodyIndex :type Integer) (bFromSweep :type Boolean) (SweepResult :type Hit%20Result%20Structure%20%28by%20ref%29))
  (if (and (Variables|Default|GetbDoingLeapAttack) (Ability|HasAuthority))
    (bind _asprimalcharacter (Utilities|Casting|CastToPrimalCharacter OtherActor))
    (if (and (!= _asprimalcharacter (Variables|Default|GetRider)) (!= _asprimalcharacter self))
      (CallFunction|FinishLeapAttack)
      (if (Class|PrimalCharacter|IsAlive)
        (bind (_outdamage _outdamagetype) (CallFunction|AddWeaponDamage (Variables|Default|GetLeapAttackDirectDamage) (Variables|Default|GetLeapDamageType) false))
        (Utilities|IsValid OtherActor
          (:Is%20Valid
            (Game|Damage|ApplyDamage OtherActor (* _outdamage (Class|PrimalCharacterStatusComponent|GetMeleeDamageModifier (Variables|Default|GetMyCharacterStatusComponent))) (Pawn|GetController) self _outdamagetype (Variables|Default|GetLeapDamageImpulse)))
          (:Is%20Not%20Valid
            _))
        (CallFunction|PlayLeapAttackHitFX)))))

(event Custom|PlayLeapAttackHitFX
  (bind _returnvalue (Transformation|GetActorLocation))
  (bind _returnvalue_2 (Transformation|GetActorRotation))
  (bind _leapattackhitfxoffset (Variables|Default|GetLeapAttackHitFXOffset))
  (bind _returnvalue_3 (Math|Vector|RotateVector _leapattackhitfxoffset _returnvalue_2))
  (bind _returnvalue_4 (+ _returnvalue _returnvalue_3))
  (bind _returnvalue_5 (Effects|SpawnEmitteratLocation (Variables|Default|GetLeapAttackHitFX) _returnvalue_4))
  (Transformation|SetRelativeScale3D _returnvalue_5 (Variables|Default|GetLeapStrikeFXScale))
  (Audio|PlaySoundatLocation (Variables|Default|GetLeapAttackHitSound) _returnvalue_4))

(event Custom|AnimNotify_CycleWeights
  (Class|PrimalDinoCharacter|CycleAttackWeightsforAttackatIndex))

(event Custom|AnimNotify_GroundLanding
  (bind _capsulecomponent (Variables|Default|GetCapsuleComponent))
  ;[1 1 1] Landing Effects
  (if (not (Networking|IsDedicatedServer))
    (bind _returnvalue (Transformation|GetWorldLocation _capsulecomponent))
    (bind (_outhit _returnvalue_2) (Class|VictoryCore|VTraceSingleBP (Class|Actor|GetWorld) _returnvalue (|OffsetFromBottomOfCapsule _capsulecomponent -2e+01 _returnvalue) "ECC_GameTraceChannel11" 0 "None" false self))
    (if _returnvalue_2
      (Utilities|FlowControl|Sequence
        (:then_0
          (bind _returnvalue_3 (Effects|SpawnEmitteratLocation (Variables|Default|GetLeapEndLandFX) (+ (.Location (Collision|BreakHitResult _outhit)) (* (Transformation|GetActorForwardVector) 75.0))))
          (Transformation|SetWorldScale3D _returnvalue_3 (Variables|Default|GetLeapEndLandFXScale)))
        (:then_1
          (Audio|PlaySoundatLocation (Variables|Default|GetLeapEndLandSound) (.Location (Collision|BreakHitResult _outhit))))))))

(event Custom|MulticastApplyLeapDownForce
  ;[1 1 1] Multicast so clients simulate added physics as well.  To reduce position teleporting.
  (Utilities|IsValid (Pawn|GetController)
    (:Is%20Valid
      (Physics|AddImpulse (Variables|Character|GetCharacterMovement) (Math|Vector|MakeVector 0.0 0.0 (Variables|Default|GetLeapFallAddedImpulse)) true 0.55))))

(event Custom|StartLeapLoopSound
  (bind _leaploop (Variables|Default|GetLeapLoop))
  (if (not (Networking|IsDedicatedServer))
    (Audio|Components|Audio|SetSound _leaploop "/Game/ScorchedEarth/Dinos/Mantis/Sounds/Mantis_Attack_Leap_Loop_Cue.Mantis_Attack_Leap_Loop_Cue")
    (Audio|Components|Audio|FadeIn _leaploop 0.4 1.0 0.0 :!class /Script/Engine.AudioComponent)))

(event EventBeginPlay
  (Utilities|FlowControl|Sequence
    (:then_0
      (Utilities|FlowControl|Delay 0.2)
      (Utilities|SwitchNetAuthority
        (:DedicatedServer
          _)
        (:PlayerServer
          _))
      (bind _asshootergamemode (Utilities|Casting|CastToShooterGameMode (Game|GetGameMode)))
      (bind _returnvalue (Class|ShooterGameMode|GetFloatOptionIni _asshootergamemode "DinoHunter" "MaxMantises"))
      (if (<= (Math|Float|Floor _returnvalue) 0)
        (Variables|Default|SetMaxAllowed 5)
        (else
          (Variables|Default|SetMaxAllowed (Math|Float|Floor _returnvalue))))
      (bind _outactors (Actor|GetAllActorsOfClass "HunterMantis_Character_BP_C"))
      (for (_ _array_index) _outactors
        (if (not (< _array_index (Variables|Default|GetMaxAllowed)))
          (Actor|DestroyActor))))))

(fn ConstructionScript
  (|CallParentFunction))

(fn BlueprintAdjustOutputDamage
  (params (AttackIndex :type Integer) (OriginalDamageAmount :type Float%20%28single-precision%29) (HitActor :type Actor%20Object%20Reference))
  (bind _attackinfos (Variables|Default|GetAttackInfos))
  (bind _item (Utilities|Array|Get(acopy) _attackinfos AttackIndex))
  (bind (_attackname _attackweight _attackrange _minattackrange _activateattackrange _attackinterval _bhighqualityattack _bskipuntamed _bskiptamed _bonlyonwilddinos _bpreventwhenencumbered _bridingonlyallowonground _bridingonlyallowwhileflying _bonlyusewithplayersorriders _bonlyusewithplayers _bpreventwhenswimming _bpreventwheninsufficientstamina _bskiponflyers _bskipai _bpreventonfemale _bpreventonmale _bpreventwhendinocarrying _buseblueprintcanriderattack _brequireswalking _brequiresswimming _attackstatusstarted _battackstopsmovement _battackstopsmovementallowfalling _battackwithjump _blocationbasedattack _bdropcarriedcharacter _bcancelanddropifcarriedcharacter _bpreventattackwhilerunning _forceupdateinrange _forceupdatemeshself _busesecondaryanimationinair _buseblueprintcanattack _buseblueprintadjustoutputdamage _bdisablerunningwhenattacking _bkeepexecutingwhenacquiringtarget _bpreventwithrider _baiforceattackdotproductcheck _binstantlyharvestcorpse _baddpawnvelocitytoprojectile _battackstopsrotation _btamedaispecialattack _bpreventwhencarryingexplosive _ballowwhenanimationpreventsinput _brequirelineofsight _busesecondaryanimationwhenswimming _busetertiaryanimationwhenswimming _bhighqualityattackonlyplayerortamed _childstateindexes _attackwithjumpchance _lastattacktime _riderlastattacktime _attackselectionexpirationtime _attackselectiontime _attackrotationrangedegrees _attackrotationgroundspeedmultiplier _attackrotationrate _meleeswingsockets _rangedsocket _meleedamageamount _meleedamageimpulse _meleeswingradius _meleedamagetype) (Utilities|Struct|BreakDinoAttackInfo _item))
  (Utilities|IsValid HitActor
    (:Is%20Valid
      (if (and (Variables|Default|GetbHasRider) (Variables|Default|GetbDoingLeapAttack))
        (CallFunction|FinishLeapAttack))
      (LocalVariables|SetbConsumeDurability true :!label _label))
    (:Is%20Not%20Valid
      (if (> (Class|VictoryCore|TimeSince (Class|Actor|GetWorld) (Variables|Default|GetLastItemDurabilityConsumedTime)) (Variables|Default|GetItemDurabilityConsumeInverval))
        (goto _label)
        (else
          (LocalVariables|SetbConsumeDurability false)))))
  (bind (_outdamage _outdamagetype) (CallFunction|AddWeaponDamage OriginalDamageAmount _meleedamagetype (LocalVariables|GetbConsumeDurability)))
  (return _outdamagetype _meleedamageimpulse _outdamage))

(fn BlueprintAnimNotifyCustomEvent
  (params (CustomEventName :type Name :default "None") (MeshComp :type Skeletal%20Mesh%20Component%20Object%20Reference) (Animation :type Anim%20Sequence%20Base%20Object%20Reference) (AnimNotifyObject :type Anim%20Notify%20Object%20Reference))
  (if (and (Networking|IsServer) (Utilities|Name|Equal(Name) CustomEventName "LeapAttackBegin"))
    (CallFunction|StartLeapAttack)))

(fn OnLanded
  (params (Hit :type Hit%20Result%20Structure%20%28by%20ref%29))
  (Development|PrintString "LANDED!")
  (if (Variables|Default|GetbDoingLeapAttack)
    (CallFunction|FinishLeapAttack)
    (return)))

(fn FinishLeapAttack
  (bind _self self)
  (bind _charactermovement (Variables|Character|GetCharacterMovement))
  (Audio|Components|Audio|FadeOut (Variables|Default|GetLeapLoop) 1.5 0.0 :!class /Script/Engine.AudioComponent)
  (Collision|SetCollisionEnabled (Variables|Default|GetAttackCheckSphere) "NoCollision")
  (Variables|Default|SetAICombatRotationRateModifier 1.0)
  (if (Class|Actor|IsDead)
    (if (Variables|Default|GetbDoingLeapAttack)
      (Variables|Default|SetbDoingLeapAttack false false))
    (Utilities|Time|ClearTimerbyFunctionName self "CheckLeapAttackEnd")
    (else
      (Class|PrimalCharacter|StopAnimEx "/Game/ScorchedEarth/Dinos/Mantis/Animations/Mantis_Attack_Leap_Montage.Mantis_Attack_Leap_Montage" false false 0.0)
      (Class|PrimalCharacter|PlayAnimEx "/Game/ScorchedEarth/Dinos/Mantis/Animations/Mantis_Attack_Leap_Out_Montage.Mantis_Attack_Leap_Out_Montage" 1.0 "None" false false false false)
      (Components|Movement|StopMovementImmediately _charactermovement)
      (Pawn|Components|CharacterMovement|SetMovementMode _charactermovement "MOVE_Falling" 0)
      (if (Ability|HasAuthority)
        (Utilities|FlowControl|Sequence
          (:then_0
            (if (Variables|Default|GetbDoingLeapAttack)
              (Variables|Default|SetbDoingLeapAttack false false))
            (Networking|ForceNetUpdate)
            (Game|Damage|ApplyRadialDamage (Variables|Default|GetLeapAttackRadiusDamage) (+ (Transformation|GetActorLocation) (Math|Vector|RotateVector (Variables|Default|GetLeapAttackDamageOffset) (Transformation|GetActorRotation))) (Variables|Default|GetLeapAttackRadius) "/Game/PrimalEarth/CoreBlueprints/DamageTypes/DmgType_Melee_Dino_Carnivore_Medium.DmgType_Melee_Dino_Carnivore_Medium_C" (Utilities|Array|MakeArray _self (Variables|Default|GetRider)) _self (Pawn|GetController) true "ECC_GameTraceChannel11" 0.0))
          (:then_1
            (Utilities|Time|ClearTimerbyFunctionName self "CheckLeapAttackEnd")))))))

(fn OnRepBDoingLeapAttack
  (Utilities|FlowControl|Sequence
    (:then_1
      (if (and (not (Variables|Default|GetbDoingLeapAttack)) (not (Ability|HasAuthority)))
        (CallFunction|FinishLeapAttack)))))

(fn AddWeaponDamage
  (params (OriginalDamage :type Float%20%28single-precision%29) (OriginalDamageType :type Damage%20Type%20Class%20Reference) (ConsumeWeaponDurability :type Boolean))
  (bind _myinventorycomponent (Variables|Default|GetMyInventoryComponent))
  (LocalVariables|SetNewDamageType OriginalDamageType)
  (Utilities|IsValid _myinventorycomponent
    (:Is%20Valid
      (bind _returnvalue (Class|PrimalInventoryComponent|GetEquippedItemOfType _myinventorycomponent "Gloves"))
      (Utilities|IsValid _returnvalue
        (:Is%20Valid
          (bind _returnvalue_2 (Class|VictoryCore|GetClassDefaultObject (Variables|/Script/ShooterGame.PrimalItem|GetWeaponTemplate _returnvalue)))
          (bind _asshooterweapon (Utilities|Casting|CastToShooterWeapon _returnvalue_2)
            (:then
              (bind _returnvalue_3 (Class|PrimalItem|GetItemStatModifier _returnvalue "WeaponDamagePercent"))
              (LocalVariables|SetNewDamage (* (Math|Conversions|ToFloat(Integer) (Variables|/Script/ShooterGame.ShooterWeapon|GetMeleeDamageAmount _asshooterweapon)) (+ (* (Variables|Default|GetWeaponAdditionalDamageMultiplier) (+ _returnvalue_3 -1.0)) 1.0)))
              (LocalVariables|SetNewDamageType (Variables|/Script/ShooterGame.ShooterWeapon|GetMeleeDamageType _asshooterweapon))
              (if ConsumeWeaponDurability
                (Class|PrimalItem|AddItemDurability _returnvalue (* (Variables|/Script/ShooterGame.ShooterWeapon|GetItemDurabilityToConsumePerMeleeHit _asshooterweapon) -1.0))
                (Variables|Default|SetLastItemDurabilityConsumedTime (Utilities|Time|GetGameTimeinSeconds))))
            (:CastFailed
              _)))
        (:Is%20Not%20Valid
          _)))
    (:Is%20Not%20Valid
      _))
  (return (+ OriginalDamage (LocalVariables|GetNewDamage)) (LocalVariables|GetNewDamageType)))

(fn BPNotifyBumpedPawn
  (params (BumpedPawn :type Primal%20Character%20Object%20Reference))
  (if (Math|Boolean|ANDBoolean (Variables|Default|GetbDoingLeapAttack) (Ability|HasAuthority) (not (Class|Actor|IsDead)))
    (bind _asprimalcharacter (Utilities|Casting|CastToPrimalCharacter BumpedPawn))
    (if (and (!= _asprimalcharacter (Variables|Default|GetRider)) (!= _asprimalcharacter self))
      (CallFunction|FinishLeapAttack)
      (bind (_outdamage _outdamagetype) (CallFunction|AddWeaponDamage (Variables|Default|GetLeapAttackDirectDamage) (Variables|Default|GetLeapDamageType) false))
      (Game|Damage|ApplyDamage BumpedPawn (* _outdamage (Class|PrimalCharacterStatusComponent|GetMeleeDamageModifier (Variables|Default|GetMyCharacterStatusComponent))) (Pawn|GetController) self _outdamagetype (Variables|Default|GetLeapDamageImpulse))
      (CallFunction|PlayLeapAttackHitFX))))

(fn BlueprintOverrideHarvestDamageType
  (bind _myinventorycomponent (Variables|Default|GetMyInventoryComponent))
  (LocalVariables|SetHarvestDamageType "/Game/PrimalEarth/CoreBlueprints/DamageTypes/DmgType_Melee_MantisHarvest.DmgType_Melee_MantisHarvest_C")
  (LocalVariables|SetMultiplier 1.0)
  (Utilities|IsValid _myinventorycomponent
    (:Is%20Valid
      (bind _returnvalue (Class|PrimalInventoryComponent|GetEquippedItemOfType _myinventorycomponent "Gloves"))
      (Utilities|IsValid _returnvalue
        (:Is%20Valid
          (LocalVariables|SetHarvestDamageType (Class|PrimalItem|GetWeaponTemplateHarvestDamageType _returnvalue))
          (LocalVariables|SetMultiplier (Class|PrimalItem|GetWeaponTemplateHarvestDamageMultiplier _returnvalue)))
        (:Is%20Not%20Valid
          _)))
    (:Is%20Not%20Valid
      _))
  (return (LocalVariables|GetMultiplier) (LocalVariables|GetHarvestDamageType)))

(fn CheckLeapAttackEnd
  (bind _returnvalue (Transformation|GetActorLocation))
  (bind _charactermovement (Variables|Character|GetCharacterMovement))
  (bind (_x _y _z) (Math|Vector|BreakVector _returnvalue))
  (bind _movementmode (Variables|/Script/Engine.CharacterMovementComponent|GetMovementMode _charactermovement))
  (bind _returnvalue_2 (Collision|LineTraceByChannel (Math|Vector|MakeVector _x _y _z) (Math|Vector|MakeVector _x _y (- _z 2e+02)) "ECC_GameTraceChannel11" false 0 "None"))
  (if _returnvalue_2
    _
    (else
      (CallFunction|MulticastApplyLeapDownForce)))
  (if (>= (Math|Conversions|ToFloat(Integer) (- (Utilities|Time|GetGameTimeinSeconds) (Variables|Default|GetStartLeapTime))) (Variables|Default|GetMaxLeapTime))
    (Pawn|Components|CharacterMovement|SetMovementMode (Variables|Character|GetCharacterMovement) "MOVE_Falling" 0)
    (Variables|Default|SetbDoingLeapAttack false false)
    (CallFunction|FinishLeapAttack :!label _label)
    (elif (and (Variables|Default|GetbDoingLeapAttack) (Ability|HasAuthority))
      (if (Math|Boolean|ORBoolean (Utilities|Enum|Equal(Enum) _movementmode "MOVE_Walking") (Utilities|Enum|Equal(Enum) _movementmode "MOVE_Swimming") (Variables|Default|GetbIsDead))
        (goto _label)))))

(fn StartLeapAttack
  (bind _returnvalue (Transformation|GetActorLocation))
  (bind _target (Variables|Default|GetTarget))
  (bind _leapattackimpulseforward (Variables|Default|GetLeapAttackImpulseForward))
  (bind _charactermovement (Variables|Character|GetCharacterMovement))
  (bind (_x _y _z) (Math|Vector|BreakVector _returnvalue))
  (bind (_x_2 _y_2 _z_2) (Math|Vector|BreakVector _returnvalue))
  (bind _returnvalue_2 (Transformation|GetActorLocation _target))
  (bind _returnvalue_3 (- _returnvalue_2 _returnvalue))
  (bind _returnvalue_4 (Math|Vector|Normalize _returnvalue_3))
  (bind _returnvalue_5 (* _returnvalue_4 _leapattackimpulseforward))
  (bind (_x_3 _y_3 _z_3) (Math|Vector|BreakVector _returnvalue_5))
  (CallFunction|StartLeapLoopSound)
  (Variables|Default|SetStartLeapTime (Utilities|Time|GetGameTimeinSeconds))
  (Variables|Default|SetStartLeapLocation (Transformation|GetActorLocation))
  (if (Ability|HasAuthority)
    (bind (_outhit _returnvalue_6) (Collision|LineTraceByChannel (Math|Vector|MakeVector _x_2 _y_2 _z_2) (Math|Vector|MakeVector _x _y (- _z 1e+03)) "ECC_WorldStatic" false 0 "None"))
    (Utilities|IsValid (Variables|Default|GetRider)
      (:Is%20Valid
        (Variables|/Script/Engine.MovementComponent|SetVelocity _charactermovement "0, 0, 0")
        (Class|PrimalCharacter|BPNetAddCharacterMovementImpulse (Math|Vector|MakeVector (.X (Math|Vector|BreakVector (* (Math|Vector|SelectVector (Math|Vector|Normalize (* (Math|Vector|CrossProduct (.ImpactNormal (Collision|BreakHitResult _outhit)) (Transformation|GetActorRightVector)) -1.0)) (Transformation|GetActorForwardVector) _returnvalue_6) (Variables|Default|GetLeapAttackImpulseForward)))) (.Y (Math|Vector|BreakVector (* (Math|Vector|SelectVector (Math|Vector|Normalize (* (Math|Vector|CrossProduct (.ImpactNormal (Collision|BreakHitResult _outhit)) (Transformation|GetActorRightVector)) -1.0)) (Transformation|GetActorForwardVector) _returnvalue_6) (Variables|Default|GetLeapAttackImpulseForward)))) (Math|Float|Min(Float) (Math|Float|SelectFloat (* (.Z (Math|Vector|BreakVector (* (Math|Vector|SelectVector (Math|Vector|Normalize (* (Math|Vector|CrossProduct (.ImpactNormal (Collision|BreakHitResult _outhit)) (Transformation|GetActorRightVector)) -1.0)) (Transformation|GetActorForwardVector) _returnvalue_6) (Variables|Default|GetLeapAttackImpulseForward)))) (Variables|Default|GetZLeapMultiplier)) (.Z (Math|Vector|BreakVector (* (Math|Vector|SelectVector (Math|Vector|Normalize (* (Math|Vector|CrossProduct (.ImpactNormal (Collision|BreakHitResult _outhit)) (Transformation|GetActorRightVector)) -1.0)) (Transformation|GetActorForwardVector) _returnvalue_6) (Variables|Default|GetLeapAttackImpulseForward)))) (>= (.Z (Math|Vector|BreakVector (* (Math|Vector|SelectVector (Math|Vector|Normalize (* (Math|Vector|CrossProduct (.ImpactNormal (Collision|BreakHitResult _outhit)) (Transformation|GetActorRightVector)) -1.0)) (Transformation|GetActorForwardVector) _returnvalue_6) (Variables|Default|GetLeapAttackImpulseForward)))) 0.0)) 0.0)) true 0.55 true "MOVE_Flying" false false))
      (:Is%20Not%20Valid
        (Utilities|IsValid _target
          (:Is%20Valid
            (Variables|/Script/Engine.MovementComponent|SetVelocity _charactermovement "0, 0, 0")
            (Class|PrimalCharacter|BPNetAddCharacterMovementImpulse (Math|Vector|MakeVector _x_3 _y_3 (Math|Float|Min(Float) (Math|Float|SelectFloat (* _z_3 (Variables|Default|GetZLeapMultiplier)) _z_3 (>= _z_3 0.0)) 0.0)) true 0.55 true "MOVE_Flying" false false))
          (:Is%20Not%20Valid
            (Variables|/Script/Engine.MovementComponent|SetVelocity _charactermovement "0, 0, 0")
            (Class|PrimalCharacter|BPNetAddCharacterMovementImpulse (Math|Vector|MakeVector (.X (Math|Vector|BreakVector (* (Math|Vector|SelectVector (Math|Vector|Normalize (* (Math|Vector|CrossProduct (.ImpactNormal (Collision|BreakHitResult _outhit)) (Transformation|GetActorRightVector)) -1.0)) (Transformation|GetActorForwardVector) _returnvalue_6) (Variables|Default|GetLeapAttackImpulseForward)))) (.Y (Math|Vector|BreakVector (* (Math|Vector|SelectVector (Math|Vector|Normalize (* (Math|Vector|CrossProduct (.ImpactNormal (Collision|BreakHitResult _outhit)) (Transformation|GetActorRightVector)) -1.0)) (Transformation|GetActorForwardVector) _returnvalue_6) (Variables|Default|GetLeapAttackImpulseForward)))) (Math|Float|Min(Float) (Math|Float|SelectFloat (* (.Z (Math|Vector|BreakVector (* (Math|Vector|SelectVector (Math|Vector|Normalize (* (Math|Vector|CrossProduct (.ImpactNormal (Collision|BreakHitResult _outhit)) (Transformation|GetActorRightVector)) -1.0)) (Transformation|GetActorForwardVector) _returnvalue_6) (Variables|Default|GetLeapAttackImpulseForward)))) (Variables|Default|GetZLeapMultiplier)) (.Z (Math|Vector|BreakVector (* (Math|Vector|SelectVector (Math|Vector|Normalize (* (Math|Vector|CrossProduct (.ImpactNormal (Collision|BreakHitResult _outhit)) (Transformation|GetActorRightVector)) -1.0)) (Transformation|GetActorForwardVector) _returnvalue_6) (Variables|Default|GetLeapAttackImpulseForward)))) (>= (.Z (Math|Vector|BreakVector (* (Math|Vector|SelectVector (Math|Vector|Normalize (* (Math|Vector|CrossProduct (.ImpactNormal (Collision|BreakHitResult _outhit)) (Transformation|GetActorRightVector)) -1.0)) (Transformation|GetActorForwardVector) _returnvalue_6) (Variables|Default|GetLeapAttackImpulseForward)))) 0.0)) 0.0)) true 0.55 true "MOVE_Flying" false false)))))
    (Variables|Default|SetbDoingLeapAttack true false)
    (Networking|ForceNetUpdate)
    (Collision|SetCollisionEnabled (Variables|Default|GetAttackCheckSphere) "QueryOnly")
    (Variables|Default|SetOldUpdateLeapTime (Utilities|Time|GetGameTimeinSeconds))
    (Variables|Default|SetAICombatRotationRateModifier 0.0)))

(fn BPCanNotifyTeamAggroAI
  (params (Dino :type Primal%20Dino%20Character%20Object%20Reference))
  (return (and (not (Class|PrimalDinoCharacter|BPIsTamed)) (Utilities|ClassIsChildOf (Utilities|GetClass Dino) "/Game/ScorchedEarth/Dinos/Mantis/Mantis_Character_BP.Mantis_Character_BP_C"))))

(fn BPShouldLimitForwardDirection
  (return (Variables|Default|GetbDoingLeapAttack)))

(fn BPTimerServer
  (CallFunction|UpdateMantisState))

(fn UpdateMantisState
  (if (Networking|IsServer)
    (if (and (Class|VictoryCore|IsTimeSince (Class|Actor|GetWorld) (Variables|Default|GetOldUpdateLeapTime) 0.2 true) (Variables|Default|GetbDoingLeapAttack))
      (if (Class|PrimalCharacter|IsAlive)
        (CallFunction|CheckLeapAttackEnd)))))

(fn BPTimerNonDedicated
  (if (not (Networking|IsServer))
    (Variables|Default|SetClientLocationInterpSpeed (select (Variables|Default|GetbDoingLeapAttack) 1e+02 5.0))))

(fn BPModifyForwardDirectionInput
  (params (directionInput :type Vector%20%28by%20ref%29 :default "0, 0, 0"))
  (return "0, 0, 0"))
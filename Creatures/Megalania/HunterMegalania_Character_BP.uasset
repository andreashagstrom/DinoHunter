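; Hunter Megalania creature Blueprint: a climbing dino variant with DinoHunter INI-configurable health, melee damage and population cap.
; On BeginPlay, authority scales the stats, and servers make the instance destroy itself when the class count exceeds MaxMegalanias.
; Rider and AI attack checks redirect the primary attack according to submersion, movement and climbing state.
; Climbing overrides filter surface normals, set trace distances and drive clamped front/back IK blendspace axes.
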(event EventBeginPlay
  (Utilities|FlowControl|Sequence
    (:then_0
      (Utilities|FlowControl|Delay 0.2)
      (Networking|SwitchHasAuthority
        (:Authority
          (bind _asshootergamemode (Utilities|Casting|CastToShooterGameMode (Game|GetGameMode)))
          ;[0 1 0.04734] Health
          (bind _returnvalue (Class|ShooterGameMode|GetFloatOptionIni _asshootergamemode "DinoHunter" "Health"))
          (if (>= _returnvalue 1.0)
            (if (<= _returnvalue 1e+03)
              (Variables|Default|SetHealth _returnvalue)
              (else
                (Variables|Default|SetHealth 1.0 :!label _label)))
            (else
              (goto _label)))
          (bind _returnvalue_2 (Class|PrimalCharacter|GetCharacterStatusComponent))
          (Class|PrimalCharacterStatusComponent|SetMaxStatusValue _returnvalue_2 "Health" (* (Class|PrimalCharacterStatusComponent|BPGetMaxStatusValue _returnvalue_2 "Health") (Variables|Default|GetHealth)))
          (Class|PrimalCharacterStatusComponent|ModifyCurrentStatusValue _returnvalue_2 "Health" (* (Class|PrimalCharacterStatusComponent|BPGetMaxStatusValue _returnvalue_2 "Health") (Variables|Default|GetHealth)) false false false false 0 false false)
          ;[1 0.01528 0] Damage
          (bind _returnvalue_3 (Class|ShooterGameMode|GetFloatOptionIni _asshootergamemode "DinoHunter" "Damage"))
          (if (>= _returnvalue_3 1.0)
            (if (<= _returnvalue_3 1e+03)
              (Variables|Default|SetDamage _returnvalue_3)
              (else
                (Variables|Default|SetDamage 1.0 :!label _label_2)))
            (else
              (goto _label_2)))
          (bind _returnvalue_4 (Class|PrimalCharacter|GetCharacterStatusComponent))
          (Class|PrimalCharacterStatusComponent|SetMaxStatusValue _returnvalue_4 "MeleeDamageMultiplier" (* (Class|PrimalCharacterStatusComponent|BPGetMaxStatusValue _returnvalue_4 "MeleeDamageMultiplier") (Variables|Default|GetDamage))))))
    (:then_1
      (|CallParentFunction)
      (Variables|Default|SetDistanceFromWaterSurfaceToAllowClimbing (* (Variables|/Script/Engine.CapsuleComponent|GetCapsuleHalfHeight (Variables|Default|GetCapsuleComponent)) 1.5)))
    (:then_2
      (Utilities|FlowControl|Delay 0.2)
      (Utilities|SwitchNetAuthority
        (:DedicatedServer
          _)
        (:PlayerServer
          _))
      (bind _asshootergamemode_2 (Utilities|Casting|CastToShooterGameMode (Game|GetGameMode)))
      (bind _returnvalue_5 (Class|ShooterGameMode|GetFloatOptionIni _asshootergamemode_2 "DinoHunter" "MaxMegalanias"))
      (if (<= (Math|Float|Floor _returnvalue_5) 0)
        (Variables|Default|SetMaxAllowed 5)
        (else
          (Variables|Default|SetMaxAllowed (Math|Float|Floor _returnvalue_5))))
      (bind _outactors (Actor|GetAllActorsOfClass "HunterMegalania_Character_BP_C"))
      (for (_ _array_index) _outactors
        (if (not (< _array_index (Variables|Default|GetMaxAllowed)))
          (Actor|DestroyActor))))))

(fn ConstructionScript
  (|CallParentFunction))

(fn BlueprintCanRiderAttack
  (params (AttackIndex :type Integer))
  (LocalVariables|SetretVal false)
  (if (< AttackIndex (Utilities|Array|Length (Variables|Default|GetAttackInfos)))
    (Utilities|FlowControl|Sequence
      (:then_0
        (switch int AttackIndex
          (:0
            (if (Class|PrimalCharacter|IsSubmerged false false false false)
              (bind _returnvalue (Class|PrimalDinoCharacter|CanAttack 4))
              (if _returnvalue
                (Class|PrimalDinoCharacter|DoAttack 4 true))
              (elif (> (Math|Vector|VectorLength (Class|PrimalDinoCharacter|GetDinoVelocity)) 0.0)
                (LocalVariables|SetretVal true)
                (else
                  (bind _result (CallFunction|IsClimberClimbing true false false false))
                  (if _result
                    (bind _returnvalue_2 (Class|PrimalDinoCharacter|CanAttack 2))
                    (if _returnvalue_2
                      (Class|PrimalDinoCharacter|DoAttack 2 true))
                    (else
                      (bind _result_2 (CallFunction|IsClimberAttaching false))
                      (if (not _result_2)
                        (bind _returnvalue_3 (Class|PrimalDinoCharacter|CanAttack 3))
                        (if _returnvalue_3
                          (Class|PrimalDinoCharacter|DoAttack 3 true)))))))))
          (:1
            (CallFunction|OnSeekPressed true))))
      (:then_1
        (return (LocalVariables|GetretVal))))
    (else
      (return (LocalVariables|GetretVal)))))

(fn BlueprintCanAttack
  (params (AttackIndex :type Integer) (distance :type Float%20%28single-precision%29) (attackRangeOffset :type Float%20%28single-precision%29) (OtherTarget :type Actor%20Object%20Reference))
  (LocalVariables|SetretVal false)
  (Utilities|FlowControl|Sequence
    (:then_0
      (if (== AttackIndex 0)
        (if (Class|PrimalCharacter|IsSubmerged false false false false)
          (bind _returnvalue (Class|PrimalDinoCharacter|CanAttack 4))
          (if _returnvalue
            (Class|PrimalDinoCharacter|DoAttack 4 true))
          (elif (> (Math|Vector|VectorLength (Class|PrimalDinoCharacter|GetDinoVelocity)) 0.0)
            (LocalVariables|SetretVal true)
            (else
              (bind _result (CallFunction|IsClimberClimbing true false false false))
              (if _result
                (bind _returnvalue_2 (Class|PrimalDinoCharacter|CanAttack 3))
                (if _returnvalue_2
                  (Class|PrimalDinoCharacter|DoAttack 3 true))
                (else
                  (bind _returnvalue_3 (Class|PrimalDinoCharacter|CanAttack 4))
                  (if _returnvalue_3
                    (Class|PrimalDinoCharacter|DoAttack 4 true)
                    (else
                      (LocalVariables|SetretVal true))))))))))
    (:then_1
      (return (LocalVariables|GetretVal)))))

(fn CheckforPreventStopClimbing
  (params (traceHitsArray :type Array%20of%20Booleans) (numValidHits :type Integer) (numTraces :type Integer))
  (return (>= numValidHits 1)))

(fn IsNormalClimbable
  (params (normal :type Vector :default "0, 0, 0") (isAverageNormal :type Boolean))
  (bind _returnvalue (Math|Vector|DotProduct normal "0, 0,1.000000"))
  (LocalVariables|SetretVal true)
  (Utilities|FlowControl|Sequence
    (:then_0
      (if (Variables|Default|GetbHasRider)
        (if (Utilities|Enum|Equal(Enum) (Variables|Default|GetCurrentClimberState_Base) "NewEnumerator13")
          (if isAverageNormal :!label _label
            (LocalVariables|SetretVal (<= _returnvalue (Variables|Default|GetRequiredNormalDotToClimb_AverageTrace)))
            (else
              (LocalVariables|SetretVal (<= _returnvalue (Variables|Default|GetrequiredNormalDotToClimb_MAX))))))
        (else
          (goto _label))))
    (:then_1
      (return (LocalVariables|GetretVal)))))

(fn GetCustomSurfaceTraceDistance
  (params (traceIndex :type Integer))
  (bind _result (CallFunction|IsClimberClimbing false false false false))
  (return (Math|Float|SelectFloat (Utilities|Array|Get(acopy) (Variables|Default|GetTraceMap_CustomTraceDistances) traceIndex) 0.0 _result)))

(fn GetClimbingIKBlendspaceAxesFront
  (bind _climbingik_maxaxisclamp (Variables|Default|GetClimbingIK_MaxAxisClamp))
  (bind _currclimbingblendspacesaxes_front (Variables|Default|GetCurrClimbingBlendspacesAxes_Front))
  (bind (_x _y) (Math|Vector2D|BreakVector2D _currclimbingblendspacesaxes_front))
  (bind _returnvalue (* _climbingik_maxaxisclamp -1.0))
  (return (Math|Vector2D|MakeVector2D (Math|Float|Clamp(Float) _x _returnvalue _climbingik_maxaxisclamp) (Math|Float|Clamp(Float) _y _returnvalue _climbingik_maxaxisclamp))))

(fn ClimbingIKSetNewBlendspaceAxes
  (bind _climbingik_canupdateaxesabovedottosurfacenormal (Variables|Default|GetClimbingIK_CanUpdateAxesAboveDotToSurfaceNormal))
  (bind _climbingik_currentmeshbenddotproducts (Variables|Default|GetClimbingIK_CurrentMeshBendDotProducts))
  (bind _climbingik_maxdottosurfacenormal (Variables|Default|GetClimbingIK_MaxDotToSurfaceNormal))
  (bind _item (Utilities|Array|Get(acopy) _climbingik_currentmeshbenddotproducts))
  (bind _item_2 (Utilities|Array|Get(acopy) _climbingik_currentmeshbenddotproducts 1))
  (bind _turndir (CallFunction|GetClimbingTurnDirection))
  (Variables|Default|SetCurrClimbingBlendspacesAxes_Front (Math|Vector2D|MakeVector2D (Math|Float|SelectFloat (- 1.0 (/ (Math|Conversions|ToFloat(Integer) _turndir) 2.0)) 0.0 (Utilities|Enum|Equal(Enum) (Variables|Default|GetCurrentClimberState_Base) "NewEnumerator12")) (/ (Math|Float|SelectFloat 0.0 _item (< (Math|Float|Absolute(Float) _item) _climbingik_canupdateaxesabovedottosurfacenormal)) _climbingik_maxdottosurfacenormal)))
  (Variables|Default|SetClimbingIK_CurrentBlendspaceAxes_Back (Math|Vector2D|MakeVector2D 0.0 (/ (Math|Float|SelectFloat 0.0 _item_2 (< (Math|Float|Absolute(Float) _item_2) _climbingik_canupdateaxesabovedottosurfacenormal)) _climbingik_maxdottosurfacenormal))))
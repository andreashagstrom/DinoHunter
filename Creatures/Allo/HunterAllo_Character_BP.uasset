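; Hunter Allo creature Blueprint, an Allo variant that scales its stats and limits its population from DinoHunter INI options on spawn.
; Shortly after BeginPlay, the authority multiplies max health and melee damage by range-checked multipliers and raises current health.
; In parallel, dedicated and player servers count all Hunter Allos, and the new one destroys itself when the count exceeds MaxAllos, which defaults to five.
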(event `self.ReceiveBeginPlay`
  (`|ExecutionSequence`
    (:`then_0`
      (`KismetSystemLibrary.Delay` 0.2)
      (`/Engine/EditorBlueprintResources/ActorMacros.Switch Has Authority`
        (:`Authority`
          (bind _asshootergamemode (cast `ShooterGameMode` (`GameplayStatics.GetGameMode`)))
          ;[0 1 0.04734] Health
          (bind _returnvalue (`ShooterGameMode.GetFloatOptionIni` _asshootergamemode "DinoHunter" "Health"))
          (if (>= _returnvalue 1.0)
            (if (<= _returnvalue 1000.0)
              (set `self.Health` _returnvalue)
              (else
                (set `self.Health` 1.0 :!label _label)))
            (else
              (goto _label)))
          (bind _returnvalue_2 (`self.GetCharacterStatusComponent`))
          (bind _returnvalue_3 (* (`PrimalCharacterStatusComponent.BPGetMaxStatusValue` _returnvalue_2 "Health") (`self.Health`)))
          (`PrimalCharacterStatusComponent.SetMaxStatusValue` _returnvalue_2 "Health" _returnvalue_3)
          (`PrimalCharacterStatusComponent.ModifyCurrentStatusValue` _returnvalue_2 "Health" _returnvalue_3 false false false false null false false)
          ;[1 0.01528 0] Damage
          (bind _returnvalue_4 (`ShooterGameMode.GetFloatOptionIni` _asshootergamemode "DinoHunter" "Damage"))
          (if (>= _returnvalue_4 1.0)
            (if (<= _returnvalue_4 1000.0)
              (set `self.Damage` _returnvalue_4)
              (else
                (set `self.Damage` 1.0 :!label _label_2)))
            (else
              (goto _label_2)))
          (bind _returnvalue_5 (`self.GetCharacterStatusComponent`))
          (`PrimalCharacterStatusComponent.SetMaxStatusValue` _returnvalue_5 "MeleeDamageMultiplier" (* (`PrimalCharacterStatusComponent.BPGetMaxStatusValue` _returnvalue_5 "MeleeDamageMultiplier") (`self.Damage`))))))
    (:`then_1`
      (`KismetSystemLibrary.Delay` 0.2)
      (`/Engine/EditorBlueprintResources/ActorMacros.SwitchNetAuthority`
        (:`DedicatedServer`
          _)
        (:`PlayerServer`
          _))
      (bind _asshootergamemode_2 (cast `ShooterGameMode` (`GameplayStatics.GetGameMode`)))
      (bind _returnvalue_6 (`ShooterGameMode.GetFloatOptionIni` _asshootergamemode_2 "DinoHunter" "MaxAllos"))
      (bind _returnvalue_7 (`KismetMathLibrary.FFloor` _returnvalue_6))
      (if (<= _returnvalue_7 0)
        (set `self.MaxAllowed` 5)
        (else
          (set `self.MaxAllowed` _returnvalue_7)))
      (bind _outactors (`GameplayStatics.GetAllActorsOfClass` "HunterAllo_Character_BP_C"))
      (for (_ _array_index) _outactors
        (if (not (< _array_index (`self.MaxAllowed`)))
          (`self.K2_DestroyActor`))))))

(fn `UserConstructionScript`
  (`parent.UserConstructionScript`))
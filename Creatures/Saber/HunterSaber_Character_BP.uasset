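; Hunter Saber creature that enforces a server-wide population cap and scales the resources it harvests.
; Shortly after BeginPlay on a dedicated or player server, it reads MaxSabers from the DinoHunter ini section, with a fallback default.
; It counts all actors of its class and destroys itself if they exceed that cap.
; Harvest quantities are multiplied by per-class scales matched through parallel resource-type and scale arrays.
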(event EventBeginPlay
  (Utilities|FlowControl|Delay 0.2)
  (Utilities|SwitchNetAuthority
    (:DedicatedServer
      _)
    (:PlayerServer
      _))
  (bind _asshootergamemode (Utilities|Casting|CastToShooterGameMode (Game|GetGameMode)))
  (bind _returnvalue (Class|ShooterGameMode|GetFloatOptionIni _asshootergamemode "DinoHunter" "MaxSabers"))
  (if (<= (Math|Float|Floor _returnvalue) 0)
    (Variables|Default|SetMaxAllowed 5)
    (else
      (Variables|Default|SetMaxAllowed (Math|Float|Floor _returnvalue))))
  (bind _outactors (Actor|GetAllActorsOfClass "HunterSaber_Character_BP_C"))
  (for (_ _array_index) _outactors
    (if (not (< _array_index (Variables|Default|GetMaxAllowed)))
      (Actor|DestroyActor))))

(fn ConstructionScript
  (|CallParentFunction))

(fn BPModifyHarvestingQuantity
  (params (originalQuantity :type Float%20%28single-precision%29) (resourceSelected :type Primal%20Item%20Class%20Reference))
  (LocalVariables|SetAmountOut originalQuantity)
  (Utilities|FlowControl|Sequence
    (:then_0
      (bind _returnvalue (Class|VictoryCore|IsChildOfClasses resourceSelected (Variables|Default|GetResourceTypesToScale)))
      (if (!= _returnvalue -1)
        (LocalVariables|SetAmountOut (* (LocalVariables|GetAmountOut) (Utilities|Array|Get(acopy) (Variables|Default|GetResourceTypeScales) _returnvalue)))))
    (:then_1
      (return (LocalVariables|GetAmountOut)))))